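; BP_Projectile is a short-lived projectile that damages third-person characters and expires after a few seconds.
; Its sphere overlap reacts only to BP_ThirdPersonCharacter actors, skipping any that share the instigator's controller so the shooter is not hit.
; On a valid hit it applies damage credited to the instigator's controller, spawns an explosion particle effect and destroys itself.
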(event OnComponentBeginOverlap(Sphere)
  (params (OverlappedComponent :type Primitive%20Component%20Object%20Reference) (OtherActor :type Actor%20Object%20Reference) (OtherComp :type Primitive%20Component%20Object%20Reference) (OtherBodyIndex :type Integer) (bFromSweep :type Boolean) (SweepResult :type Hit%20Result%20Structure%20%28by%20ref%29))
  (bind _instigator (Variables|Actor|GetInstigator))
  (bind _returnvalue (Pawn|GetController _instigator))
  (bind _asbp_third_person_character (Utilities|Casting|CastToBP_ThirdPersonCharacter OtherActor))
  (if (!= (Pawn|GetController _asbp_third_person_character) _returnvalue)
    (Game|Damage|ApplyDamage OtherActor 1e+01 _returnvalue self)
    (Effects|SpawnEmitteratLocation "/Game/StarterContent/Particles/P_Explosion.P_Explosion" (Transformation|GetActorLocation))
    (Actor|DestroyActor)))

(event EventBeginPlay
  (Actor|SetLifeSpan 3.0))

(fn ConstructionScript)