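; BP_Door is a stage door that swings between closed and open.
; Open and Close set IsOpen, and OnRep_isOpen responds by calling OpenAnim or CloseAnim with animation on.
; A Timeline plays or reverses to scale the Door component's relative yaw toward 100 degrees or back.
; Both animation events can also snap straight to the end rotation when animation is off.
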(event Custom|Open
  (Variables|Default|SetisOpen true))

(event Custom|OpenAnim
  (params (animation :type Boolean))
  (bind _door (Variables|Default|GetDoor))
  (if animation
    (bind _rate (Timeline|Timeline Play)
      (:Update
        (Transformation|SetRelativeRotation _door (* (Math|Rotator|MakeRotator 0.0 0.0 1e+02) _rate) false false)))
    (else
      (Transformation|SetRelativeRotation _door (Math|Rotator|MakeRotator 0.0 0.0 1e+02) false false))))

(event Custom|Close
  (Variables|Default|SetisOpen false))

(event Custom|CloseAnim
  (params (animation :type Boolean))
  (bind _door (Variables|Default|GetDoor))
  (if animation
    (bind _rate (Timeline|Timeline Reverse)
      (:Update
        (Transformation|SetRelativeRotation _door (* (Math|Rotator|MakeRotator 0.0 0.0 1e+02) _rate) false false)))
    (else
      (Transformation|SetRelativeRotation _door (Math|Rotator|MakeRotator 0.0 0.0 0.0) false false))))

(fn ConstructionScript)

(fn OnRepIsOpen
  (if (Variables|Default|GetisOpen)
    (CallFunction|OpenAnim true)
    (else
      (CallFunction|CloseAnim true))))