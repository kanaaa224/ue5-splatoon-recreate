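; Main HUD for the Splatoon-style game, managing the in-game, pause and match result screens.
; BeginPlay creates Widget_Main and adds it to the viewport.
; Tick polls GameState_Main for IsTimeUp, then once swaps the main widget for Widget_MatchResult.
; The Pause event adds a pause menu widget; both it and the result screen switch input to UI-only with a visible cursor.
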(event Custom|Pause
  (bind _returnvalue (Game|Player|GetOwningPlayerController))
  (bind _returnvalue_2 (UserInterface|CreateWidget "/Game/Splatoon/Menu/Blueprints/Widget_PauseMenu.Widget_PauseMenu_C"))
  (bind _output_get (Variables|Default|SetpauseMenuWidgetRef _returnvalue_2))
  (UserInterface|Viewport|AddtoViewport _output_get 0)
  (Input|SetInputModeUIOnly _returnvalue 0 "DoNotLock" false)
  (Variables|/Script/Engine.PlayerController|SetbShowMouseCursor _returnvalue true))

(event EventBeginPlay
  (Utilities|FlowControl|Sequence
    (:then_0
      (bind _returnvalue (UserInterface|CreateWidget "/Game/Splatoon/System/Blueprints/Widget_Main.Widget_Main_C" (Game|Player|GetOwningPlayerController)))
      (bind _output_get (Variables|Default|SetwidgetRef _returnvalue))
      (UserInterface|Viewport|AddtoViewport _output_get 0))))

(event EventTick
  (params (DeltaSeconds :type Float%20%28single-precision%29))
  (bind _returnvalue (Game|Player|GetOwningPlayerController))
  (bind _asgame_state_main (Utilities|Casting|CastToGameState_Main (Game|GetGameState)))
  (if (Variables|/Game/Splatoon/System/Blueprints/GameState_Main.GameState_Main_C|GetIsTimeUp _asgame_state_main)
    (Utilities|FlowControl|DoOnce false
      (:Completed
        (Widget|RemovefromParent (Variables|Default|GetwidgetRef))
        (bind _returnvalue_2 (UserInterface|CreateWidget "/Game/Splatoon/Player/Blueprints/Widget_MatchResult.Widget_MatchResult_C" _returnvalue))
        (UserInterface|Viewport|AddtoViewport _returnvalue_2 0)
        (Input|SetInputModeUIOnly _returnvalue 0 "DoNotLock" false)
        (Variables|/Script/Engine.PlayerController|SetbShowMouseCursor _returnvalue true)))))

(fn ConstructionScript)