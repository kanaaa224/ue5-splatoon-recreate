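; GameState_Main is the game state Blueprint that exposes the match countdown and current player count.
; GetTimeLeft subtracts the time elapsed since MatchStartDateTime from TimeLeft and returns minutes and seconds, so the countdown is derived on demand rather than ticked.
; GetCurrentPlayersNum derives the count from the last loop index over PlayerArray.
; The TimeLeft RepNotify, event graph and construction script are empty.
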(event EventBeginPlay)

(event EventTick
  (params (DeltaSeconds :type Float%20%28single-precision%29)))

(fn ConstructionScript)

(fn OnRepTimeLeft)

(fn GetTimeLeft
  (bind _returnvalue (Math|DateTime|Now))
  (bind _matchstartdatetime (Variables|Default|GetMatchStartDateTime))
  (bind _timeleft (Variables|Default|GetTimeLeft))
  (bind _returnvalue_2 (- _returnvalue _matchstartdatetime))
  (bind _returnvalue_3 (- _timeleft _returnvalue_2))
  (return (Math|Timespan|GetMinutes _returnvalue_3) (Math|Timespan|GetSeconds _returnvalue_3)))

(fn GetCurrentPlayersNum
  (for (_ _array_index) (Variables|Default|GetPlayerArray)
    _)
  (return (+ _array_index 1)))